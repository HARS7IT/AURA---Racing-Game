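; BP_Checkpoint is a race checkpoint that tracks a sports car's progress through an ordered course.
; When a BP_VehicleAdvSportsCar overlaps its Cube, it compares its Index with the car's last crossed checkpoint plus one.
; The correct next checkpoint records itself and its index on the car and calls Finish if flagged as the finish line.
; Skipped or repeated checkpoints only print a message.
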(event `self.Cube.OnComponentBeginOverlap`
  (params (OverlappedComponent :type "PrimitiveComponent Object Reference") (OtherActor :type "Actor Object Reference") (OtherComp :type "PrimitiveComponent Object Reference") (OtherBodyIndex :type Integer) (bFromSweep :type Boolean) (SweepResult :type "HitResult Structure (by ref)"))
  (bind _index (`self.Index`))
  (bind _asbp_vehicle_adv_sports_car (cast `/Game/VehicleTemplate/Blueprints/SportsCar/BP_VehicleAdvSportsCar` OtherActor))
  (`/Engine/EditorBlueprintResources/StandardMacros.CompareInt` _index (+ (`/Game/VehicleTemplate/Blueprints/SportsCar/BP_VehicleAdvSportsCar.CheckpointCrossed` _asbp_vehicle_adv_sports_car) 1)
    (:`>`
      (`KismetSystemLibrary.PrintString` "You are missing checkpoint"))
    (:`==`
      (set `/Game/VehicleTemplate/Blueprints/SportsCar/BP_VehicleAdvSportsCar.CheckpointCrossed` _index _asbp_vehicle_adv_sports_car)
      (set `/Game/VehicleTemplate/Blueprints/SportsCar/BP_VehicleAdvSportsCar.lastcheckpoint` self _asbp_vehicle_adv_sports_car)
      (if (`self.IsFinishLine`)
        (`/Game/VehicleTemplate/Blueprints/SportsCar/BP_VehicleAdvSportsCar.finish` _asbp_vehicle_adv_sports_car)))
    (:`<`
      (`KismetSystemLibrary.PrintString` "You have already been here"))))

(fn `UserConstructionScript`)